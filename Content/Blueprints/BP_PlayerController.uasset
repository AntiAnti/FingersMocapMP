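; Player controller that creates the main UI frame, adds the global input mapping context, and switches between camera modes.
; SetCameraMode updates the existing camera pawn's mode for the preset views.
; Switching to or from Free mode destroys the pawn and spawns and possesses the matching camera pawn class at the same transform.
; The free camera uses game-and-UI input, while preset views use UI-only input with the cursor shown.
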(event Custom|SetCameraMode
  (params (Mode :type E_CameraMode%20Enum :default "NewEnumerator0"))
  (if (Utilities|Enum|NotEqual(Enum) Mode (Variables|Default|GetCameraMode))
    (Variables|Default|SetPawnTransform (Transformation|GetActorTransform (Pawn|GetControlledPawn)))
    (Utilities|FlowControl|Sequence
      (:then_0
        (switch Utilities|FlowControl|Switch|SwitchonE_CameraMode Mode
          (:NewEnumerator0
            (if (Utilities|Enum|Equal(Enum) (Variables|Default|GetCameraMode) "NewEnumerator3") :!label _label
              (Utilities|RespawnCamera "/Game/Blueprints/BP_CameraPawn.BP_CameraPawn_C" false)
              (else
                (bind _asbp_camera_pawn (Utilities|Casting|CastToBP_CameraPawn (Pawn|GetControlledPawn)))
                (Variables|/Game/Blueprints/BP_CameraPawn.BP_CameraPawn_C|SetMode _asbp_camera_pawn Mode))))
          (:NewEnumerator1
            (goto _label))
          (:NewEnumerator2
            (goto _label))
          (:NewEnumerator3
            (if (not (Utilities|Enum|Equal(Enum) (Variables|Default|GetCameraMode) "NewEnumerator3"))
              (Utilities|RespawnCamera "/Game/Blueprints/BP_FreeCameraPawn.BP_FreeCameraPawn_C" true)))))
      (:then_1
        (Variables|Default|SetCameraMode Mode)))))

(event EventBeginPlay
  (bind _returnvalue (UserInterface|CreateWidget "/Game/UI/W_MainFrame.W_MainFrame_C" self))
  (bind _output_get (Variables|Default|SetUIFrame _returnvalue))
  (UserInterface|Viewport|AddtoViewport _output_get 0)
  (Input|AddMappingContext (PlayerController|LocalPlayerSubsystems|GetEnhancedInputLocalPlayerSubsystem) "/Game/Input/IM_Global.IM_Global" 0 "(bIgnoreAllPressedKeysUntilRelease=True,bForceImmediately=False)")
  (Input|SetInputModeUIOnly self (Variables|Default|GetUIFrame) "DoNotLock" false)
  (Variables|Default|SetbShowMouseCursor true))

(fn ConstructionScript)