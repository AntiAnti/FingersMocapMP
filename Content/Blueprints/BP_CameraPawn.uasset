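; Camera pawn that automatically frames the hands of the body mesh from BP_HandObserver.
; After a short delay on BeginPlay it caches the observer's mesh and hand bone names, then each tick builds a pivot between both hands and measures their separation.
; Cam Target To Hands derives front, back and far-front transforms scaled by that separation; Mode selects one, and the pawn eases toward it with TInterpTo.
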(event EventBeginPlay
  (Utilities|FlowControl|Delay 0.2)
  (bind _returnvalue (Actor|GetActorOfClass "/Game/Blueprints/BP_HandObserver.BP_HandObserver_C"))
  (bind _output_get (Variables|Default|SetHandObserver _returnvalue))
  (Variables|Default|SetHandBoneRight (Variables|/Script/MediapipeFingers.FingerDataExtractorComponent|GetHandBoneRight (Variables|/Game/Blueprints/BP_HandObserver.BP_HandObserver_C|GetFingerDataExtractor _output_get)))
  (Variables|Default|SetHandBoneLeft (Variables|/Script/MediapipeFingers.FingerDataExtractorComponent|GetHandBoneLeft (Variables|/Game/Blueprints/BP_HandObserver.BP_HandObserver_C|GetFingerDataExtractor _output_get)))
  (Variables|Default|SetBodyMesh (Variables|/Game/Blueprints/BP_HandObserver.BP_HandObserver_C|GetBodyMesh (Variables|Default|GetHandObserver))))

(event EventTick
  (params (DeltaSeconds :type Float%20%28single-precision%29))
  (bind (_front _back _frontfar) (|CamTargetToHands))
  (bind _handboneright (Variables|Default|GetHandBoneRight))
  (bind _handboneleft (Variables|Default|GetHandBoneLeft))
  (bind _bodymesh (Variables|Default|GetBodyMesh))
  (bind _returnvalue (Transformation|GetSocketLocation _bodymesh _handboneleft))
  (bind _returnvalue_2 (Transformation|GetSocketLocation _bodymesh _handboneright))
  (bind _returnvalue_3 (- _returnvalue_2 _returnvalue))
  (Utilities|IsValid _bodymesh
    (:Is%20Valid
      (Variables|Default|SetDT DeltaSeconds)
      (Variables|Default|SetHandsDistance (Math|Vector|VectorLength _returnvalue_3))
      (Variables|Default|SetMeshPivot (Math|Transform|MakeTransform (* (+ _returnvalue_2 _returnvalue) 0.5) (Class|KismetMathLibrary|MakeRotfromYZ _returnvalue_3 (Transformation|GetActorUpVector))))
      (Utilities|FlowControl|Sequence
        (:then_0
          (switch Utilities|FlowControl|Switch|SwitchonE_CameraMode (Variables|Default|GetMode)
            (:NewEnumerator0
              (Variables|Default|SetCameraTarget _front))
            (:NewEnumerator1
              (Variables|Default|SetCameraTarget _back))
            (:NewEnumerator2
              (Variables|Default|SetCameraTarget _frontfar))))
        (:then_1
          (Transformation|SetActorLocationAndRotation (.location (Class|KismetMathLibrary|TInterpto (Transformation|GetActorTransform) (Variables|Default|GetCameraTarget) (Variables|Default|GetDT) 2.0)) (.rotation (Class|KismetMathLibrary|TInterpto (Transformation|GetActorTransform) (Variables|Default|GetCameraTarget) (Variables|Default|GetDT) 2.0))))))))

(fn ConstructionScript)