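; BP_FreeCameraPawn is a pawn that works as a free-flying camera controlled through Enhanced Input.
; IA_WASD adds movement input along the camera's forward and right vectors, so forward movement follows the view direction.
; IA_Mouse feeds controller yaw and pitch, with the vertical axis inverted before it is applied.
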(event Input|EnhancedActionEvents|EnhancedInputActionIA_WASD
  (params (ActionValue :type Vector%202D%20Structure) (ElapsedSeconds :type Float%20%28double-precision%29) (TriggeredSeconds :type Float%20%28double-precision%29) (InputAction :type Input%20Action%20Object%20Reference :default "/Game/Input/IA_WASD.IA_WASD"))
  (bind (_x _y) (Math|Vector2D|BreakVector2D ActionValue))
  (bind _camera (Variables|Default|GetCamera))
  (:Triggered
    (Pawn|Input|AddMovementInput (+ (* (Math|Vector|GetForwardVector _camera) _x) (* (Math|Vector|GetRightVector _camera) _y)) 1.0 false)))

(event Input|EnhancedActionEvents|EnhancedInputActionIA_Mouse
  (params (ActionValue :type Vector%202D%20Structure) (ElapsedSeconds :type Float%20%28double-precision%29) (TriggeredSeconds :type Float%20%28double-precision%29) (InputAction :type Input%20Action%20Object%20Reference :default "/Game/Input/IA_Mouse.IA_Mouse"))
  (bind (_x _y) (Math|Vector2D|BreakVector2D ActionValue))
  (:Triggered
    (Pawn|Input|AddControllerYawInput _x)
    (Pawn|Input|AddControllerPitchInput (* _y -1.0))))

(event EventBeginPlay)

(fn ConstructionScript)