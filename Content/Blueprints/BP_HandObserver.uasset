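; BP_HandObserver is an actor that previews and manages finger animation data from FingerDataExtractor on a mannequin body mesh.
; Each tick it feeds both hands' preview states into FK/IK finger solvers and caches MediaPipe-style landmarks from Observer.
; Extractor events update the player controller's UI, while keyframes and the filter interval are drawn to a timeline render target.
; It also saves and restores extractor projects through BP_AnimationSaveGame slots.
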(event OnTime(FingerDataExtractor)
  (params (Time :type Float%20%28single-precision%29) (Frame :type Integer64))
  (Variables|Default|SetAnimTime Time)
  (bind _asbp_player_controller (Utilities|Casting|CastToBP_PlayerController (Game|GetPlayerController 0)))
  (Default|OnPlayTime (Variables|/Game/Blueprints/BP_PlayerController.BP_PlayerController_C|GetUIFrame _asbp_player_controller) (Variables|Default|GetAnimTime) false))

(event OnStop(FingerDataExtractor)
  (bind _asbp_player_controller (Utilities|Casting|CastToBP_PlayerController (Game|GetPlayerController 0)))
  (Default|OnStop (Variables|/Game/Blueprints/BP_PlayerController.BP_PlayerController_C|GetUIFrame _asbp_player_controller)))

(event OnAnimationUpdated(FingerDataExtractor)
  (bind _asbp_player_controller (Utilities|Casting|CastToBP_PlayerController (Game|GetPlayerController 0)))
  (CallFunction|UpdateKeyframesCanvas)
  (Default|UpdateAnimationData (Variables|/Game/Blueprints/BP_PlayerController.BP_PlayerController_C|GetUIFrame _asbp_player_controller)))

(event Custom|SaveData
  (params (FileName :type String))
  (bind _returnvalue (SaveGame|CreateSaveGameObject "/Game/Blueprints/BP_AnimationSaveGame.BP_AnimationSaveGame_C"))
  (Default|FillfromObject _returnvalue (Variables|Default|GetFingerDataExtractor))
  (SaveGame|SaveGametoSlot _returnvalue FileName))

(event Custom|LoadData
  (params (FileName :type String))
  (bind _returnvalue (SaveGame|LoadGamefromSlot FileName))
  (bind _asbp_animation_save_game (Utilities|Casting|CastToBP_AnimationSaveGame _returnvalue))
  (Class|FingerDataExtractorComponent|RestoreProject (Variables|Default|GetFingerDataExtractor) (Variables|/Game/Blueprints/BP_AnimationSaveGame.BP_AnimationSaveGame_C|GetAnimationData _asbp_animation_save_game) (Variables|/Game/Blueprints/BP_AnimationSaveGame.BP_AnimationSaveGame_C|GetAnimationIntervals _asbp_animation_save_game) (Variables|/Game/Blueprints/BP_AnimationSaveGame.BP_AnimationSaveGame_C|GetAnimationKeyFrames _asbp_animation_save_game)))

(event Custom|UpdateKeyframesCanvas
  (bind (_canvas _size _context) (Rendering|BeginDrawCanvastoRenderTarget "/Game/Materials/Textures/T_KeyFramesBackground.T_KeyFramesBackground"))
  (Class|Canvas|DrawLine _canvas "(X=-32.000000,Y=32.000000)" "(X=544.000000,Y=32.000000)" 64.0 "(R=0.000000,G=0.000000,B=0.000000,A=1.000000)")
  (for _array_element (Class|FingerDataExtractorComponent|GetAnimationKeyFrames (Variables|Default|GetFingerDataExtractor))
    (Class|Canvas|DrawLine _canvas (Math|Vector2D|MakeVector2D (Utilities|TimetoCanvasX (Class|FingerDataExtractorComponent|GetTimeatFrame (Variables|Default|GetFingerDataExtractor) (Math|Conversions|ToInteger(Byte) (.Frame (Utilities|Struct|BreakFingersKeyframe _array_element))))) 0.0) (Math|Vector2D|MakeVector2D (Utilities|TimetoCanvasX (Class|FingerDataExtractorComponent|GetTimeatFrame (Variables|Default|GetFingerDataExtractor) (Math|Conversions|ToInteger(Byte) (.Frame (Utilities|Struct|BreakFingersKeyframe _array_element))))) 32.0) 2.0 "(R=0.000000,G=0.361111,B=1.000000,A=1.000000)"))
  (Utilities|DrawIntervalonCanvas _canvas)
  (Rendering|EndDrawCanvastoRenderTarget _context))

(event Custom|UpdateFilterIntervalCanvas
  (bind (_canvas _size _context) (Rendering|BeginDrawCanvastoRenderTarget "/Game/Materials/Textures/T_KeyFramesBackground.T_KeyFramesBackground"))
  (Class|Canvas|DrawLine _canvas "(X=0.000000,Y=48.000000)" "(X=544.000000,Y=48.000000)" 3e+01 "(R=0.000000,G=0.000000,B=0.000000,A=1.000000)")
  (Utilities|FlowControl|Sequence
    (:then_0
      (Utilities|DrawIntervalonCanvas _canvas))
    (:then_1
      (Rendering|EndDrawCanvastoRenderTarget _context))))

(event EventBeginPlay
  (|CallParentFunction)
  (Utilities|FlowControl|Delay 0.2)
  (bind _returnvalue (Class|FingersFKIKSolver|CreateFingersFKIKSolver "/Game/FingersSetup/Mannequin_RightHand.Mannequin_RightHand" (Variables|Default|GetBodyMesh)))
  (bind _output_get (Variables|Default|SetFingerSolverRight _returnvalue))
  (Class|FingersFKIKSolver|ResetFingersPose _output_get)
  (bind _returnvalue_2 (Class|FingersFKIKSolver|CreateFingersFKIKSolver "/Game/FingersSetup/Mannequin_LeftHand.Mannequin_LeftHand" (Variables|Default|GetBodyMesh)))
  (bind _output_get_2 (Variables|Default|SetFingerSolverLeft _returnvalue_2))
  (Class|FingersFKIKSolver|ResetFingersPose _output_get_2))

(event Collision|EventActorBeginOverlap
  (params (OtherActor :type Actor%20Object%20Reference)))

(event EventTick
  (params (DeltaSeconds :type Float%20%28single-precision%29))
  (|CallParentFunction DeltaSeconds)
  (Utilities|IsValid (Variables|Default|GetFingerSolverRight)
    (:Is%20Valid
      (Utilities|FlowControl|Sequence
        (:then_0
          (|DrawDebug))
        (:then_2
          (Class|FingersFKIKSolver|ApplyVRInputRaw (Variables|Default|GetFingerSolverRight) (Variables|/Script/MediapipeFingers.FingerDataExtractorComponent|GetPreviewStateRight (Variables|Default|GetFingerDataExtractor)))
          (Class|FingersFKIKSolver|ApplyVRInputRaw (Variables|Default|GetFingerSolverLeft) (Variables|/Script/MediapipeFingers.FingerDataExtractorComponent|GetPreviewStateLeft (Variables|Default|GetFingerDataExtractor)))
          (Class|FingersFKIKSolver|UpdateFingers (Variables|Default|GetFingerSolverLeft) false true))))))

(fn ConstructionScript
  (|CallParentFunction))