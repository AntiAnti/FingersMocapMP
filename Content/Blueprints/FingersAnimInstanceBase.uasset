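; FingersAnimInstanceBase is a base animation instance for finger animation on a BP_HandObserver actor.
; On update it lazily caches the observer's EditAnimation, left and right finger solvers and finger data extractor from the owning actor.
; Once cached, it sets Alpha to fully on or off depending on whether the extractor has frame data.
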(event EventBlueprintUpdateAnimation
  (params (DeltaTimeX :type Float%20%28single-precision%29))
  (if (not (Math|Boolean|ANDBoolean (Utilities|IsValid (Variables|Default|GetEditAnimation)) (Utilities|IsValid (Variables|Default|GetRightSolver)) (Utilities|IsValid (Variables|Default|GetLeftSolver))))
    (bind _asbp_hand_observer (Utilities|Casting|CastToBP_HandObserver (Class|AnimInstance|GetOwningActor)))
    (Variables|Default|SetHandObserver _asbp_hand_observer)
    (Variables|Default|SetEditAnimation (Variables|/Game/Blueprints/BP_HandObserver.BP_HandObserver_C|GetEditAnimation _asbp_hand_observer))
    (Variables|Default|SetRightSolver (Variables|/Game/Blueprints/BP_HandObserver.BP_HandObserver_C|GetFingerSolverRight _asbp_hand_observer))
    (Variables|Default|SetLeftSolver (Variables|/Game/Blueprints/BP_HandObserver.BP_HandObserver_C|GetFingerSolverLeft _asbp_hand_observer))
    (Variables|Default|SetFingersData (Variables|/Game/Blueprints/BP_HandObserver.BP_HandObserver_C|GetFingerDataExtractor _asbp_hand_observer))
    (else
      (Variables|Default|SetAlpha (Math|Float|SelectFloat 1.0 0.0 (Variables|/Script/MediapipeFingers.FingerDataExtractorComponent|GetbHasFrameData (Variables|Default|GetFingersData)))))))